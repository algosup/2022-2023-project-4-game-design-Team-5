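; BP_Move is an actor Blueprint that moves its static mesh in fixed steps from keyboard input and can restart the level.
; Z, S, Q and D (AZERTY layout) each add a local offset along X or Y once per press, without sweep, so movement ignores collision.
; The Restart input action runs the RestartLevel console command.
; Tick, BeginPlay and overlap events are empty, and an actor rotation node is left unconnected.
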(event `Key|Z`
  (params (Key :type "Key Structure"))
  (:`Pressed`
    (`SceneComponent.K2_AddLocalOffset` (`self.StaticMesh`) (100.0 0.0 0.0) false false)))

(event `InputAction|Restart`
  (params (Key :type "Key Structure"))
  (:`Pressed`
    (`KismetSystemLibrary.ExecuteConsoleCommand` "RestartLevel" null)))

(event `Key|Q`
  (params (Key :type "Key Structure"))
  (:`Pressed`
    (`SceneComponent.K2_AddLocalOffset` (`self.StaticMesh`) (0.0 -100.0 0.0) false false)))

(event `Key|S`
  (params (Key :type "Key Structure"))
  (:`Pressed`
    (`SceneComponent.K2_AddLocalOffset` (`self.StaticMesh`) (-100.0 0.0 0.0) false false)))

(event `Key|D`
  (params (Key :type "Key Structure"))
  (:`Pressed`
    (`SceneComponent.K2_AddLocalOffset` (`self.StaticMesh`) (0.0 100.0 0.0) false false)))

(fn `UserConstructionScript`)