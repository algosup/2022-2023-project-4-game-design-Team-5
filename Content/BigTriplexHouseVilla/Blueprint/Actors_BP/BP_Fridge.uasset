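; Interactive fridge Blueprint whose three doors open and close on left mouse click.
; Each click toggles the Icon's visibility and plays or reverses a timeline per door, based on its current track value.
; LeftDoor and RightDoor swing on yaw, while BigDoor slides along relative Y.
; Player input enable and disable logic exists, but nothing triggers it in this graph.
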(event `Key|LeftMouseButton`
  (params (Key :type "Key Structure"))
  (:`Pressed`
    (`SceneComponent.ToggleVisibility` (`self.icon`) false)))

(event `Key|LeftMouseButton`
  (params (Key :type "Key Structure"))
  (:`Pressed`
    (if (< (stale _newtrack_0) 1.0)
      (bind (_direction _newtrack_0) (`Timeline|Timeline_2` :!label _label)
        (:`Update`
          (`SceneComponent.K2_SetRelativeRotation` (`self.LeftDoor`) (`KismetMathLibrary.MakeRotator` 0.0 0.0 _newtrack_0) false false)))
      (else
        (goto _label :!via `Reverse`)))))

(event `Key|LeftMouseButton`
  (params (Key :type "Key Structure"))
  (:`Pressed`
    (if (> (stale _newtrack_0) -1.0)
      (bind (_direction _newtrack_0) (`Timeline|Timeline_3` :!label _label_2)
        (:`Update`
          (`SceneComponent.K2_SetRelativeRotation` (`self.RightDoor`) (`KismetMathLibrary.MakeRotator` 0.0 0.0 _newtrack_0) false false)))
      (else
        (goto _label_2 :!via `Reverse`)))))

(event `Key|LeftMouseButton`
  (params (Key :type "Key Structure"))
  (:`Pressed`
    (if (> 1.0 (stale _newtrack_0))
      (bind (_direction _newtrack_0) (`Timeline|Timeline_0` :!label _label_3)
        (:`Update`
          (`SceneComponent.K2_SetRelativeTransform` (`self.BigDoor`) (`KismetMathLibrary.MakeTransform` (`KismetMathLibrary.MakeVector` 0.0 _newtrack_0)) false false)))
      (else
        (goto _label_3 :!via `Reverse`)))))

(fn `UserConstructionScript`)